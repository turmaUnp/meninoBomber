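; Sudden-death zone actor ("morte subita") that kills a BP_meninoBomber player who leaves its sphere.
; Tick, throttled by a one-second Delay, counts down Tempojogo through truncated float subtraction.
; At 30 or below, it reveals the hidden sphere and plays the Tamanhomortal timeline to drive its world scale.
; Ending overlap with the sphere at any time sets the player's Morto flag and calls MorteEHud on BP_MyGameMode.
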(event `self.ReceiveBeginPlay`
  (`SceneComponent.SetHiddenInGame` (`self.Sphere`) true false)
  (bind _asbp_my_game_mode (cast `/Game/BomberMAnClone/Bluprint/BP_MyGameMode` (`GameplayStatics.GetGameMode`)))
  (set `self.gamemode` _asbp_my_game_mode))

(event `self.ReceiveTick`
  (params (DeltaSeconds :type "Float (single-precision)"))
  (`KismetSystemLibrary.Delay` 1.0)
  (bind _output_get (set `self.tempojogo` (`KismetMathLibrary.FTrunc` (- (`KismetMathLibrary.Conv_IntToDouble` (`self.tempojogo`)) DeltaSeconds))))
  (if (<= _output_get 30)
    (`SceneComponent.SetHiddenInGame` (`self.Sphere`) false false)
    (bind (_direction _tamanho) (`Timeline|tamanhomortal`)
      (:`Update`
        (`SceneComponent.SetWorldScale3D` (`self.Sphere`) (`KismetMathLibrary.Conv_DoubleToVector` _tamanho))))))

(event `self.Sphere.OnComponentEndOverlap`
  (params (OverlappedComponent :type "PrimitiveComponent Object Reference") (OtherActor :type "Actor Object Reference") (OtherComp :type "PrimitiveComponent Object Reference") (OtherBodyIndex :type Integer))
  (bind _asbp_menino_bomber (cast `/Game/BomberMAnClone/BomberPlayer/BP_meninoBomber` OtherActor))
  (set `/Game/BomberMAnClone/BomberPlayer/BP_meninoBomber.morto` true _asbp_menino_bomber)
  (`/Game/BomberMAnClone/Bluprint/BP_MyGameMode.morte e hud` (`self.gamemode`)))

(fn `UserConstructionScript`)