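; Destructible cube for a Bomberman clone that breaks when hit by an explosion and may leave a random item behind.
; Two overlap boxes each react to a different explosion class, BP_explosao_2 or BP_explosao.
; A hit picks from an eight-slot class array with four empty slots, so about half the hits spawn an item at the cube's transform.
; The cube and that explosion are then destroyed, limiting each explosion to one block.
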(event `self.ReceiveTick`
  (params (DeltaSeconds :type "Float (single-precision)")))

(event `self.Box.OnComponentBeginOverlap`
  (params (OverlappedComponent :type "PrimitiveComponent Object Reference") (OtherActor :type "Actor Object Reference") (OtherComp :type "PrimitiveComponent Object Reference") (OtherBodyIndex :type Integer) (bFromSweep :type Boolean) (SweepResult :type "HitResult Structure (by ref)"))
  ;[1 1 1] explode um bloco por vez
  (bind _asbp_explosao_2 (cast `/Game/BomberMAnClone/Bomba/BP_explosao_2` OtherActor))
  (`|SpawnActorFromClass` (`|GetArrayItem` (`|MakeArray` "/Game/BomberMAnClone/Cenario/Itens/BP_bombatorre.BP_bombatorre_C" "/Game/BomberMAnClone/Cenario/Itens/BPC_patins.BPC_patins_C" "/Game/BomberMAnClone/Cenario/Itens/BPC_fogo.BPC_fogo_C" "/Game/BomberMAnClone/Cenario/Itens/BPC_cabum.BPC_cabum_C" null null null null :!type "Actor Class Reference") (`KismetMathLibrary.RandomIntegerInRange` 0 7)) (`SceneComponent.K2_GetComponentToWorld` (`self.DefaultSceneRoot`)) "Undefined" "OverrideRootScale")
  (`self.K2_DestroyActor`)
  (`self.K2_DestroyActor` _asbp_explosao_2))

(event `self.Box1.OnComponentBeginOverlap`
  (params (OverlappedComponent :type "PrimitiveComponent Object Reference") (OtherActor :type "Actor Object Reference") (OtherComp :type "PrimitiveComponent Object Reference") (OtherBodyIndex :type Integer) (bFromSweep :type Boolean) (SweepResult :type "HitResult Structure (by ref)"))
  ;[1 1 1] explode um bloco por vez
  (bind _asbp_explosao (cast `/Game/BomberMAnClone/Bomba/BP_explosao` OtherActor))
  (`|SpawnActorFromClass` (`|GetArrayItem` (`|MakeArray` "/Game/BomberMAnClone/Cenario/Itens/BP_bombatorre.BP_bombatorre_C" "/Game/BomberMAnClone/Cenario/Itens/BPC_patins.BPC_patins_C" "/Game/BomberMAnClone/Cenario/Itens/BPC_fogo.BPC_fogo_C" "/Game/BomberMAnClone/Cenario/Itens/BPC_cabum.BPC_cabum_C" null null null null :!type "Actor Class Reference") (`KismetMathLibrary.RandomIntegerInRange` 0 7)) (`SceneComponent.K2_GetComponentToWorld` (`self.DefaultSceneRoot`)) "Undefined" "OverrideRootScale" null null)
  (`self.K2_DestroyActor`)
  (`self.K2_DestroyActor` _asbp_explosao))

(fn `UserConstructionScript`)