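; BP_totem is a trigger totem on the phase 2 platform of a Bomberman clone, activated by bomb explosions.
; When a BP_explosao overlaps its Box, it finds all actors implementing the BP_pisos interface and sends CairpisoMessage with NewVar0, apparently to drop floor pieces.
; It then tints its mesh red through a dynamic material instance.
; The game mode reference cached on BeginPlay is not used in this graph.
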(event `self.ReceiveBeginPlay`
  (bind _asbp_my_game_mode (cast `/Game/BomberMAnClone/Bluprint/BP_MyGameMode` (`GameplayStatics.GetGameMode`)))
  (set `self.gamemode` _asbp_my_game_mode))

(event `self.Box.OnComponentBeginOverlap`
  (params (OverlappedComponent :type "PrimitiveComponent Object Reference") (OtherActor :type "Actor Object Reference") (OtherComp :type "PrimitiveComponent Object Reference") (OtherBodyIndex :type Integer) (bFromSweep :type Boolean) (SweepResult :type "HitResult Structure (by ref)"))
  (cast `/Game/BomberMAnClone/Bomba/BP_explosao` OtherActor)
  (bind _outactors (`GameplayStatics.GetAllActorsWithInterface` "/Game/BomberMAnClone/fases/fase2/plataforma/BP_pisos.BP_pisos_C"))
  (message `/Game/BomberMAnClone/fases/fase2/plataforma/BP_pisos.cairpiso` _outactors (`self.NewVar_0`))
  (bind _returnvalue (`PrimitiveComponent.CreateDynamicMaterialInstance` (`self.StaticMesh1`) 0 null "None"))
  (`MaterialInstanceDynamic.SetVectorParameterValue` _returnvalue "cor" (struct :`R` 0.941667 :`A` 1.0)))

(fn `UserConstructionScript`)