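; BP_armadilha is a stage 5 trap in the Bomberman clone that fires a BP_labareda flame when BP_meninoBomber enters its box.
; The overlap turns the mesh glowing yellow as a warning, then after a delay turns it red and spawns the flame at the Arrow's transform.
; After a cooldown it turns green without glow and resets the DoOnce that blocks retriggering.
; Each color change creates a dynamic material instance.
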(event `self.Box.OnComponentBeginOverlap`
  (params (OverlappedComponent :type "PrimitiveComponent Object Reference") (OtherActor :type "Actor Object Reference") (OtherComp :type "PrimitiveComponent Object Reference") (OtherBodyIndex :type Integer) (bFromSweep :type Boolean) (SweepResult :type "HitResult Structure (by ref)"))
  (cast `/Game/BomberMAnClone/BomberPlayer/BP_meninoBomber` OtherActor)
  (`/Engine/EditorBlueprintResources/StandardMacros.DoOnce` false :!label _label
    (:`Completed`
      (bind _returnvalue (`PrimitiveComponent.CreateDynamicMaterialInstance` (`self.StaticMesh`) 0 null "None"))
      (`MaterialInstanceDynamic.SetVectorParameterValue` _returnvalue "colorArmadilha" (struct :`R` 0.920833 :`G` 0.87603 :`B` 0.068421 :`A` 1.0))
      (`MaterialInstanceDynamic.SetScalarParameterValue` _returnvalue "emissiveArmadilha" 1.0)
      (`KismetSystemLibrary.Delay` 1.0)
      (`self.labareda`))))

(event `labareda`
  (bind _returnvalue (`PrimitiveComponent.CreateDynamicMaterialInstance` (`self.StaticMesh`) 0 null "None"))
  (`MaterialInstanceDynamic.SetVectorParameterValue` _returnvalue "colorArmadilha" (struct :`R` 0.920833 :`G` 0.047889 :`A` 1.0))
  (`MaterialInstanceDynamic.SetScalarParameterValue` _returnvalue "emissiveArmadilha" 2.0)
  (`KismetSystemLibrary.Delay` 0.2)
  (`|SpawnActorFromClass` "/Game/BomberMAnClone/fases/fase5/BP_labareda.BP_labareda_C" (`SceneComponent.K2_GetComponentToWorld` (`self.Arrow`)) "Undefined" "OverrideRootScale" null null)
  (`KismetSystemLibrary.Delay` 2.5)
  (bind _returnvalue_2 (`PrimitiveComponent.CreateDynamicMaterialInstance` (`self.StaticMesh`) 0 null "None"))
  (`MaterialInstanceDynamic.SetVectorParameterValue` _returnvalue_2 "colorArmadilha" (struct :`R` 0.012091 :`G` 0.920833 :`A` 1.0))
  (`MaterialInstanceDynamic.SetScalarParameterValue` _returnvalue_2 "emissiveArmadilha" 0.0)
  (goto _label :!via `Reset`))

(fn `UserConstructionScript`)