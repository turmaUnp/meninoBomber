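; BP_labareda is a moving flame hazard for stage 5 (fase5) that kills the player on contact.
; Tick moves it along its forward vector at constant speed until it is far enough from the world origin, then stops it and destroys it after a short delay.
; Box overlap with BP_meninoBomber sets its Morto flag and calls MorteEHud on the cached game mode.
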(event `self.ReceiveBeginPlay`
  (bind _asbp_my_game_mode (cast `/Game/BomberMAnClone/Bluprint/BP_MyGameMode` (`GameplayStatics.GetGameMode`)))
  (set `self.gamemode` _asbp_my_game_mode))

(event `self.ReceiveTick`
  (params (DeltaSeconds :type "Float (single-precision)"))
  (if (not (`self.stop`))
    (`self.K2_AddActorWorldOffset` (* (`self.GetActorForwardVector`) (* DeltaSeconds 300.0)))
    (if (>= (`KismetMathLibrary.VSize` (`self.K2_GetActorLocation`)) 1500.0)
      (set `self.stop` true)
      (`KismetSystemLibrary.Delay` 1.0)
      (`self.K2_DestroyActor`))))

(event `self.Box.OnComponentBeginOverlap`
  (params (OverlappedComponent :type "PrimitiveComponent Object Reference") (OtherActor :type "Actor Object Reference") (OtherComp :type "PrimitiveComponent Object Reference") (OtherBodyIndex :type Integer) (bFromSweep :type Boolean) (SweepResult :type "HitResult Structure (by ref)"))
  (bind _asbp_menino_bomber (cast `/Game/BomberMAnClone/BomberPlayer/BP_meninoBomber` OtherActor))
  (set `/Game/BomberMAnClone/BomberPlayer/BP_meninoBomber.morto` true _asbp_menino_bomber)
  (`/Game/BomberMAnClone/Bluprint/BP_MyGameMode.morte e hud` (`self.gamemode`)))

(fn `UserConstructionScript`)