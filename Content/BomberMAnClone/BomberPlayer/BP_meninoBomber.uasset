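; Player character for a Bomberman clone that drops bombs, collects power-ups, opens the pause menu and creates a shared or split-screen HUD from a GameInstance flag.
; Capsule overlaps with BP_itemMaster log the item and boost fire, walk speed or bomb capacity, or enable tower bombs.
; Bombs spawn if a per-Tick forward box trace is clear and capacity remains; the used count zeroes after a delay.
; Tick also pins the overhead camera and updates a countdown.
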(event `InputAction|Pause`
  (params (Key :type "Key Structure"))
  (:`Pressed`
    (`self.pausarGame`)))

(event `self.CapsuleComponent.OnComponentBeginOverlap`
  (params (OverlappedComponent :type "PrimitiveComponent Object Reference") (OtherActor :type "Actor Object Reference") (OtherComp :type "PrimitiveComponent Object Reference") (OtherBodyIndex :type Integer) (bFromSweep :type Boolean) (SweepResult :type "HitResult Structure (by ref)"))
  (bind _itemmaster (`self.itemMaster`))
  (bind _itemmaster_2 (`self.itemMaster`))
  (bind _itemmaster_3 (`self.itemMaster`))
  (bind _itemmaster_4 (`self.itemMaster`))
  (bind _charactermovement (`self.CharacterMovement`))
  ;[1 1 1] pegaritem
  (bind _asbp_item_master (cast `/Game/BomberMAnClone/Cenario/Itens/BP_itemMaster` OtherActor))
  (set `self.itemMaster` _asbp_item_master)
  (`GameplayStatics.PlaySoundAtLocation` "/Game/BomberMAnClone/Sons/pegarItem_Cue.pegarItem_Cue" (`SceneComponent.K2_GetComponentLocation` (`self.pontoDeExplosao`)) (struct) 1.0 1.0 0.0 null null null)
  (`self.item`)
  (`|ExecutionSequence`
    (:`then_0`
      (switch `/Game/BomberMAnClone/Cenario/Itens/Item` (`.categoria_7_4D19474240F6DCA9B25D1FA6F0274420` (break `/Game/BomberMAnClone/Cenario/Itens/Boster` (`/Game/BomberMAnClone/Cenario/Itens/BP_itemMaster.Itens` (`self.itemMaster`))))
        (:`NewEnumerator0`
          (bind _result (`/Engine/EditorBlueprintResources/StandardMacros.IncrementInt` (`self.fogoextra`))
            (:`  `
              (set `self.fogoextra` _result)
              ;[1 1 1] fogo/almenta o poder de fogo
              (set `self.maisFogo` (* (`self.maisFogo`) 2.0))
              (`/Engine/EditorBlueprintResources/StandardMacros.IsValid` _itemmaster_4
                (:`Is Valid`
                  (`self.K2_DestroyActor` _itemmaster_4))))))
        (:`NewEnumerator1`
          (bind _result_2 (`/Engine/EditorBlueprintResources/StandardMacros.IncrementInt` (`self.patins`))
            (:`  `
              (set `self.patins` _result_2)
              ;[1 1 1] Patins/adicionavelocidade
              (set `CharacterMovementComponent.MaxWalkSpeed` (+ (`CharacterMovementComponent.MaxWalkSpeed` _charactermovement) 200.0) _charactermovement)
              (`/Engine/EditorBlueprintResources/StandardMacros.IsValid` _itemmaster_2
                (:`Is Valid`
                  (`self.K2_DestroyActor` _itemmaster_2))))))
        (:`NewEnumerator2`
          (bind _result_3 (`/Engine/EditorBlueprintResources/StandardMacros.IncrementInt` (`self.bombaextra`))
            (:`  `
              (set `self.bombaextra` _result_3)
              ;[1 1 1] Bomba/adicona uma bomba
              (bind _result_4 (`/Engine/EditorBlueprintResources/StandardMacros.IncrementFloat` (`self.totalCabum`))
                (:`  `
                  (bind _output_get (set `self.totalCabum` _result_4))
                  (`KismetSystemLibrary.PrintString` (`KismetStringLibrary.Conv_DoubleToString` _output_get))
                  (`/Engine/EditorBlueprintResources/StandardMacros.IsValid` _itemmaster_3
                    (:`Is Valid`
                      (`self.K2_DestroyActor` _itemmaster_3))))))))
        (:`NewEnumerator4`
          ;[1 1 1] bomba torre
          (set `self.bombatorre` true)
          (`/Engine/EditorBlueprintResources/StandardMacros.IsValid` _itemmaster
            (:`Is Valid`
              (`self.K2_DestroyActor` _itemmaster))))))))

(event `self.ReceiveTick`
  (params (DeltaSeconds :type "Float (single-precision)"))
  (bind _returnvalue (`self.K2_GetActorLocation`))
  (bind _camera (`self.Camera`))
  ;[1 1 1] posicao da camera e tempo limite
  (`|ExecutionSequence`
    (:`then_0`
      (`SceneComponent.K2_SetRelativeLocation` _camera (0.0 0.0 608.0) false false)
      (`SceneComponent.K2_SetWorldRotation` _camera (struct :`Pitch` -60.0 :`Yaw` -90.0) false false)
      (`KismetSystemLibrary.Delay` 1.0)
      (bind _output_get (set `self.tempofinal` (`KismetMathLibrary.FTrunc` (- (`KismetMathLibrary.Conv_IntToDouble` (`self.tempofinal`)) DeltaSeconds))))
      (`KismetSystemLibrary.PrintString` (`KismetStringLibrary.Conv_IntToString` _output_get)))
    (:`then_1`
      ;[1 1 1] verificar se pode colocar bomba
      (bind (_outhit _returnvalue_2) (`KismetSystemLibrary.BoxTraceSingleForObjects` :`Start` _returnvalue :`End` (+ _returnvalue (* (`self.GetActorForwardVector`) 50.0)) :`HalfSize` (20.0 20.0 20.0) :`ObjectTypes` (`|MakeArray` "ObjectTypeQuery1" "ObjectTypeQuery1" "ObjectTypeQuery1" :!type "EObjectTypeQuery Enum") :`DrawDebugType` "ForOneFrame"))
      (set `self.podeBomba` _returnvalue_2))))

(event `InputAction|Bomba`
  (params (Key :type "Key Structure"))
  (bind (_returnvalue_location _returnvalue_rotation _returnvalue_scale) (`KismetMathLibrary.BreakTransform` (`SceneComponent.K2_GetComponentToWorld` (`self.pontoDeExplosao`))))
  ;[1 1 1] spawn Bomba e controle de quantidade
  (:`Pressed`
    (if (not (`self.podeBomba`))
      (if (< (`self.cabumusado`) (`self.totalCabum`))
        (bind _result (`/Engine/EditorBlueprintResources/StandardMacros.IncrementFloat` (`self.cabumusado`))
          (:`  `
            (set `self.cabumusado` _result)
            (if (`self.bombatorre`)
              (`|SpawnActorFromClass` "/Game/BomberMAnClone/Bomba/BP_CabumTorre.BP_CabumTorre_C" (`KismetMathLibrary.MakeTransform` _returnvalue_location (struct) _returnvalue_scale) "AlwaysSpawn" "OverrideRootScale" null null)
              (`KismetSystemLibrary.Delay` 3.0)
              (set `self.cabumusado` 0.0)
              (else
                (`|SpawnActorFromClass` "/Game/BomberMAnClone/Bomba/BP_Cabum.BP_Cabum_C" (`KismetMathLibrary.MakeTransform` _returnvalue_location (struct) _returnvalue_scale) "AlwaysSpawn" "OverrideRootScale" null null)
                (`KismetSystemLibrary.Delay` 3.0)
                (set `self.cabumusado` 0.0)))))))))

(event `self.ReceiveBeginPlay`
  ;[1 1 1] tela na hud
  (bind _asbp_my_game_instance (cast `/Game/BomberMAnClone/Blueprint/BP_myGAmeInstance` (`GameplayStatics.GetGameInstance`)))
  (if (`/Game/BomberMAnClone/Blueprint/BP_myGAmeInstance.telaCompartilhada` _asbp_my_game_instance)
    (bind _returnvalue (`|CreateWidget` "/Game/BomberMAnClone/Hud/BP_telacompartilhada.BP_telacompartilhada_C" (`GameplayStatics.GetPlayerController` 0)))
    (`UserWidget.AddToViewport` _returnvalue 0)
    (else
      (bind _returnvalue_2 (`|CreateWidget` "/Game/BomberMAnClone/Hud/BP_teladividida.BP_teladividida_C" (`GameplayStatics.GetPlayerController` 0)))
      (`UserWidget.AddToPlayerScreen` _returnvalue_2 0))))

(fn `item`
  (`KismetArrayLibrary.Array_Add` (`self.bosters`) (`/Game/BomberMAnClone/Cenario/Itens/BP_itemMaster.Itens` (`self.itemMaster`))))

(fn `pausarGame`
  (`GameplayStatics.SetGamePaused` true)
  (`/Engine/EditorBlueprintResources/StandardMacros.IsValid` (`self.menuPauseWidget`)
    (:`Is Valid`
      _)
    (:`Is Not Valid`
      (bind _returnvalue (`|CreateWidget` "/Game/BomberMAnClone/Hud/BP_PauseMenu.BP_PauseMenu_C" (`GameplayStatics.GetPlayerController` 0)))
      (bind _output_get (set `self.menuPauseWidget` _returnvalue))))
  (`UserWidget.AddToViewport` _output_get 0)
  (set `PlayerController.bShowMouseCursor` true (`GameplayStatics.GetPlayerController` 0)))

(fn `pegarItem`
  (params (NewParam3 :type "/Game/BomberMAnClone/Cenario/Itens/BP_itemMaster Object Reference"))
  (returns (ativar :type Boolean) (quantidade :type Integer) (categoria :type Byte))
  (set `self.itemMaster` NewParam3)
  (`self.item`)
  (for _array_element (`self.bosters`)
    _)
  (bind (_ativar _quatidade _categoria) (break `/Game/BomberMAnClone/Cenario/Itens/Boster` _array_element))
  (return _ativar _quatidade _categoria))

(fn `UserConstructionScript`)

(fn `voltarGame`
  (`GameplayStatics.SetGamePaused` false)
  (`Widget.RemoveFromParent` (`self.menuPauseWidget`))
  (set `PlayerController.bShowMouseCursor` false (`GameplayStatics.GetPlayerController` 0)))