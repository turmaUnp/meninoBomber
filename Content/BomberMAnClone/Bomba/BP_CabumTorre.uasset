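; BP_CabumTorre is a timed explosive in a Bomberman clone that bursts in a cross pattern.
; On BeginPlay it caches the player's BP_meninoBomber and plays the ScalaBomba timeline, which drives the static mesh's scale as a pre-detonation animation.
; When the timeline finishes, it spawns a BP_explosao_2 at AreaCabum facing each of the four horizontal axis directions, then destroys itself.
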(event `self.ReceiveBeginPlay`
  (bind _staticmesh (`self.StaticMesh`))
  (`|ExecutionSequence`
    (:`then_0`
      ;[1 1 1] pegarReferencia e limitar efeito de particulas
      (bind _asbp_menino_bomber (cast `/Game/BomberMAnClone/BomberPlayer/BP_meninoBomber` (`GameplayStatics.GetPlayerCharacter` 0)))
      (set `self.meninoBomber` _asbp_menino_bomber))
    (:`then_1`
      ;[1 1 1] explosao em cruz
      (bind (_direction _tamanho_antes_da_morte) (`Timeline|scalaBomba`)
        (:`Update`
          (`/Engine/EditorBlueprintResources/StandardMacros.IsValid` _staticmesh
            (:`Is Valid`
              (`SceneComponent.SetWorldScale3D` _staticmesh (`KismetMathLibrary.Conv_DoubleToVector` _tamanho_antes_da_morte)))))
        (:`Finished`
          (`self.explosao`))))))

(event `explosao`
  ;[1 1 1] explosao direcional
  (for _array_element (`|MakeArray` (1.0 0.0 0.0) (0.0 1.0 0.0) (-1.0 0.0 0.0) (0.0 -1.0 0.0) :!type "Vector Structure")
    (`|SpawnActorFromClass` "/Game/BomberMAnClone/Bomba/BP_explosao_2.BP_explosao_2_C" (`KismetMathLibrary.MakeTransform` (`SceneComponent.K2_GetComponentLocation` (`self.areaCabum`)) (`KismetMathLibrary.Conv_VectorToRotator` _array_element)) "Undefined" "OverrideRootScale" null null))
  (`self.K2_DestroyActor`))

(fn `UserConstructionScript`)