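; BP_CabumCopia is a movable actor in the Bomberman clone's bomb folder, steered by the player who owns it.
; On BeginPlay it casts its owner to BP_meninoBomber, gets that character's BP_MyPlayerController and binds to its forward and right move events.
; Each event applies forced movement input along fixed negative world X or Y, scaled by the axis value and MultiplicarVel.
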(event `self.ReceiveBeginPlay`
  (`parent.ReceiveBeginPlay`)
  (bind _asbp_menino_bomber (cast `/Game/BomberMAnClone/BomberPlayer/BP_meninoBomber` (`self.GetOwner`)))
  (set `/Game/BomberMAnClone/BomberPlayer/BP_meninoBomber.maisFogo` (`/Game/BomberMAnClone/BomberPlayer/BP_meninoBomber.maisFogo` _asbp_menino_bomber) _asbp_menino_bomber)
  (bind _asbp_my_player_controller (cast `/Game/BomberMAnClone/Bluprint/BP_MyPlayerController` (`self.GetController` _asbp_menino_bomber)))
  (bind _output_get (set `self.owner playercontroler` _asbp_my_player_controller))
  (add `/Game/BomberMAnClone/Bluprint/BP_MyPlayerController.moverfowardevent` _output_get (delegate `moverfoward`))
  (add `/Game/BomberMAnClone/Bluprint/BP_MyPlayerController.moverrightevent` _output_get (delegate `moveright`)))

(event `moverfoward`
  (params (axivalue1 :type "Float (double-precision)"))
  (`self.AddMovementInput` (-1.0 0.0 0.0) (* axivalue1 (`self.multiplicarVel`)) true))

(event `moveright`
  (params (axivalue :type "Float (double-precision)"))
  (`self.AddMovementInput` (0.0 -1.0 0.0) (* axivalue (`self.multiplicarVel`)) true))

(fn `UserConstructionScript`
  (`parent.UserConstructionScript`))