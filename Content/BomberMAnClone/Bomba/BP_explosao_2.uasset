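; Moving explosion blast for a Bomberman clone that kills any BP_meninoBomber it overlaps while travelling.
; On BeginPlay a forward box trace against WorldStatic shortens its fixed maximum range to the first obstacle, playing a sound on a hit.
; Tick moves it forward, with the player's MaisFogo adding speed, until it reaches that range, pauses briefly and destroys itself.
; Kills set Morto and call the GameMode's MorteEHud.
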(event `self.ReceiveBeginPlay`
  (bind _posicaoinicial (`self.posicaoinicial`))
  (`|ExecutionSequence`
    (:`then_0`
      ;[1 1 1] referencia menino bomber
      (bind _asbp_menino_bomber (cast `/Game/BomberMAnClone/BomberPlayer/BP_meninoBomber` (`GameplayStatics.GetPlayerCharacter` 0)))
      (set `self.meninoBomber` _asbp_menino_bomber)
      (bind _asbp_my_game_mode (cast `/Game/BomberMAnClone/Bluprint/BP_MyGameMode` (`GameplayStatics.GetGameMode`)))
      (set `self.gamemode` _asbp_my_game_mode))
    (:`then_1`
      ;[1 1 1] limita o alcance da explosao
      (set `self.tamanho` 900.0)
      (set `self.posicaoinicial` (`self.K2_GetActorLocation`))
      (bind (_outhit _returnvalue) (`KismetSystemLibrary.BoxTraceSingleForObjects` _posicaoinicial (+ _posicaoinicial (* (`self.GetActorForwardVector`) (`self.tamanho`))) (20.0 20.0 20.0) (struct) (`|MakeArray` "ObjectTypeQuery1" :!type "EObjectTypeQuery Enum")))
      (if _returnvalue
        (set `self.tamanho` (`.Distance` (`GameplayStatics.BreakHitResult` _outhit)))
        (`GameplayStatics.PlaySoundAtLocation` "/Game/BomberMAnClone/Sons/bomba_Cue.bomba_Cue" (`SceneComponent.K2_GetComponentLocation` (`self.Box`)) (struct) 1.0 1.0 0.0 null null null)))))

(event `self.ReceiveTick`
  (params (DeltaSeconds :type "Float (single-precision)"))
  ;[1 1 1] direção da explosao
  (if (not (`self.stop?`))
    (`self.K2_AddActorWorldOffset` (* (`self.GetActorForwardVector`) (* DeltaSeconds (+ (`self.velocidade`) (`/Game/BomberMAnClone/BomberPlayer/BP_meninoBomber.maisFogo` (`self.meninoBomber`))))))
    (if (>= (`KismetMathLibrary.VSize` (- (`self.posicaoinicial`) (`self.K2_GetActorLocation`))) (`self.tamanho`))
      (set `self.stop?` true)
      (`KismetSystemLibrary.Delay` 0.5)
      (`self.K2_DestroyActor`))))

(event `self.Box.OnComponentBeginOverlap`
  (params (OverlappedComponent :type "PrimitiveComponent Object Reference") (OtherActor :type "Actor Object Reference") (OtherComp :type "PrimitiveComponent Object Reference") (OtherBodyIndex :type Integer) (bFromSweep :type Boolean) (SweepResult :type "HitResult Structure (by ref)"))
  ;[1 1 1] mata menino bomber
  (if (not (`self.stop?`))
    (bind _asbp_menino_bomber (cast `/Game/BomberMAnClone/BomberPlayer/BP_meninoBomber` OtherActor))
    (set `/Game/BomberMAnClone/BomberPlayer/BP_meninoBomber.morto` true _asbp_menino_bomber)
    (`/Game/BomberMAnClone/Bluprint/BP_MyGameMode.morte e hud` (`self.gamemode`))))

(fn `UserConstructionScript`)