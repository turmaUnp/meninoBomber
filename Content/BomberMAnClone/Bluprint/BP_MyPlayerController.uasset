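; Player controller for a Bomberman clone that drives the possessed BP_meninoBomber and supports shared or split-screen views.
; Axis input moves the pawn along fixed world axes and fires movement events with the axis value.
; On BeginPlay it registers itself with BP_MyGameMode.
; On possess, the game instance's TelaCompartilhada flag selects either a per-player split-screen HUD or, with a valid game mode, its main camera.
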(event `InputAxis|MoveRight`
  (params (AxisValue :type "Float (single-precision)"))
  ;[1 1 1] movimentação player
  (`Pawn.AddMovementInput` (`self.meninobomber`) (1.0 0.0 0.0) AxisValue false)
  (`self.moverfowardevent` AxisValue))

(event `InputAxis|MoveForward`
  (params (AxisValue :type "Float (single-precision)"))
  ;[1 1 1] movimentação player
  (`Pawn.AddMovementInput` (`self.meninobomber`) (0.0 1.0 0.0) AxisValue false)
  (`self.moverrightevent` AxisValue))

(event `self.ReceiveBeginPlay`
  (bind _asbp_my_game_mode (cast `/Game/BomberMAnClone/Bluprint/BP_MyGameMode` (`GameplayStatics.GetGameMode`)))
  (bind _output_get (set `self.gamemode` _asbp_my_game_mode))
  (`/Game/BomberMAnClone/Bluprint/BP_MyGameMode.receberControlador` _output_get self))

(event `self.ReceivePossess`
  (params (PossessedPawn :type "Pawn Object Reference"))
  (`|ExecutionSequence`
    (:`then_0`
      (bind _asbp_my_game_instance (cast `/Game/BomberMAnClone/Bluprint/BP_myGAmeInstance` (`GameplayStatics.GetGameInstance`)))
      (if (not (`/Game/BomberMAnClone/Bluprint/BP_myGAmeInstance.telaCompartilhada` _asbp_my_game_instance))
        (bind _returnvalue (`|CreateWidget` "/Game/BomberMAnClone/Hud/BP_teladividida.BP_teladividida_C" self))
        (bind _output_get (set `self.hudTeladividida` _returnvalue))
        (`UserWidget.AddToPlayerScreen` _output_get 0)))
    (:`then_1`
      (bind _asbp_menino_bomber (cast `/Game/BomberMAnClone/BomberPlayer/BP_meninoBomber` PossessedPawn))
      (set `self.meninobomber` _asbp_menino_bomber)
      (bind _gamemode (`self.gamemode`)
        (:`then`
          (`|ExecutionSequence`
            (:`then_0`
              (if (`/Game/BomberMAnClone/Bluprint/BP_myGAmeInstance.telaCompartilhada` _asbp_my_game_instance)
                (`self.SetViewTargetWithBlend` (`/Game/BomberMAnClone/Bluprint/BP_MyGameMode.cameraPrincipal` _gamemode))))))
        (:`else`)))))

(event `self.ReceiveUnPossess`
  (params (UnpossessedPawn :type "Pawn Object Reference"))
  (set `self.meninobomber` null))

(fn `UserConstructionScript`)