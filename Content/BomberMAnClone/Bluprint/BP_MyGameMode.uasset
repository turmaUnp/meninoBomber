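; Game mode for a Bomberman clone that sets up a second local player and a choice between split and shared screen.
; On BeginPlay it applies the game instance's shared-screen flag, adding a HUD if set, then creates player 1's controller.
; Camera and controller setters each point that controller's view at the shared camera in that mode.
; MorteEHud pauses the game and shows the death menu; ChaoNochao is an empty stub.
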(event `self.ReceiveBeginPlay`
  (`|ExecutionSequence`
    (:`then_0`
      (bind _asbp_my_game_instance (cast `/Game/BomberMAnClone/Bluprint/BP_myGAmeInstance` (`GameplayStatics.GetGameInstance`)))
      (bind _output_get (set `self.gameinstance` _asbp_my_game_instance))
      (bind _telacompartilhada (`/Game/BomberMAnClone/Bluprint/BP_myGAmeInstance.telaCompartilhada` _output_get))
      (`GameplayStatics.SetForceDisableSplitscreen` _telacompartilhada)
      (if _telacompartilhada
        (bind _returnvalue (`|CreateWidget` "/Game/BomberMAnClone/Hud/BP_telacompartilhada.BP_telacompartilhada_C"))
        (bind _output_get_2 (set `self.hudTelacompartida` _returnvalue))
        (`UserWidget.AddToViewport` _output_get_2 0)))
    (:`then_1`
      (bind _returnvalue_2 (`GameplayStatics.CreatePlayer` 1))
      (bind _asbp_my_player_controller (cast `/Game/BomberMAnClone/Bluprint/BP_MyPlayerController` _returnvalue_2))
      (`self.receberControlador` _asbp_my_player_controller))))

(event `self.ReceiveTick`
  (params (DeltaSeconds :type "Float (single-precision)")))

(event `ativarplatadorma`
  (`self.chaoNochao`))

(fn `cameraPrincipal`
  (returns (NewParam :type "/Game/BomberMAnClone/Bluprint/CameraActor_Blueprint Object Reference"))
  (return (`self.camera`)))

(fn `chaoNochao`)

(fn `morte e hud`
  (`GameplayStatics.SetGamePaused` true)
  (bind _returnvalue (`|CreateWidget` "/Game/BomberMAnClone/Hud/BP_hudMorte.BP_hudMorte_C" (`GameplayStatics.GetPlayerController` 0)))
  (bind _output_get (set `self.menumorte` _returnvalue))
  (`UserWidget.AddToViewport` _output_get 0)
  (set `PlayerController.bShowMouseCursor` true (`GameplayStatics.GetPlayerController` 0))
  (`/Game/BomberMAnClone/Hud/BP_hudMorte.chamarhud` (`self.menumorte`)))

(fn `receberCamera`
  (params (NewVar_1 :type "/Game/BomberMAnClone/Bluprint/CameraActor_Blueprint Object Reference"))
  (bind _asbp_my_game_instance (cast `/Game/BomberMAnClone/Bluprint/BP_myGAmeInstance` (`GameplayStatics.GetGameInstance`)))
  (set `self.camera` NewVar_1)
  (if (`/Game/BomberMAnClone/Bluprint/BP_myGAmeInstance.telaCompartilhada` _asbp_my_game_instance)
    (`PlayerController.SetViewTargetWithBlend` (`self.playerocntroler`) (`self.camera`) 0.0 "VTBlend_Linear" 0.0 false)))

(fn `receberControlador`
  (params (`[0]` :type "/Game/BomberMAnClone/Bluprint/BP_MyPlayerController Object Reference"))
  (bind _asbp_my_game_instance (cast `/Game/BomberMAnClone/Bluprint/BP_myGAmeInstance` (`GameplayStatics.GetGameInstance`)))
  (set `self.playerocntroler` (`|MakeArray` `[0]`))
  (`|ExecutionSequence`
    (:`then_0`
      (if (`/Game/BomberMAnClone/Bluprint/BP_myGAmeInstance.telaCompartilhada` _asbp_my_game_instance)
        (bind _camera (`self.camera`)
          (:`then`
            (`PlayerController.SetViewTargetWithBlend` (`self.playerocntroler`) _camera 0.0 "VTBlend_Linear" 0.0 false))
          (:`else`))))))

(fn `UserConstructionScript`)